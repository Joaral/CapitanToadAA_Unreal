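; BP_Lock is a one-time lock that opens when a BP_ThirdPersonCharacter enters its Box while holding a BP_Key.
; The overlap sets IsUnlocked, then loops through Receivers, calling SwitchOnMessage on each.
; Key destruction, clearing of HeldObject and the lock's own destruction sit inside that loop, so they repeat per receiver and never run when Receivers is empty.
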(event OnComponentBeginOverlap(Box)
  (params (OverlappedComponent :type Primitive%20Component%20Object%20Reference) (OtherActor :type Actor%20Object%20Reference) (OtherComp :type Primitive%20Component%20Object%20Reference) (OtherBodyIndex :type Integer) (bFromSweep :type Boolean) (SweepResult :type Hit%20Result%20Structure%20%28by%20ref%29))
  (if (not (Variables|Default|GetisUnlocked))
    (bind _asbp_third_person_character (Utilities|Casting|CastToBP_ThirdPersonCharacter OtherActor))
    (bind _asbp_key (Utilities|Casting|CastToBP_Key (Variables|/Game/ThirdPerson/Blueprints/BP_ThirdPersonCharacter.BP_ThirdPersonCharacter_C|GetHeldObject _asbp_third_person_character)))
    (Variables|Default|SetisUnlocked true)
    (for _array_element (Variables|Default|GetReceivers)
      (Class|ISignalReceiver|Switchon(Message) _array_element)
      (Actor|DestroyActor _asbp_key)
      (Variables|/Game/ThirdPerson/Blueprints/BP_ThirdPersonCharacter.BP_ThirdPersonCharacter_C|SetHeldObject _asbp_third_person_character 0)
      (Actor|DestroyActor))))

(fn ConstructionScript)