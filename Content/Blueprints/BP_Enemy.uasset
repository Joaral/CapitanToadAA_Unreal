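; Enemy character that damages the player on overlap and loses health when hit by the player, using the same Damage value for both.
; AI perception writes the sensed player to the AI controller's Blackboard and clears that key when sensing is lost, also rewriting a second key with its own value.
; On death from its HealthComponent, it launches backward and is destroyed after a short delay; a spawn node is left unconnected.
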(event OnTargetPerceptionUpdated(AIPerception)
  (params (Actor :type Actor%20Object%20Reference) (Stimulus :type AI%20Stimulus%20Structure))
  (bind _returnvalue (Pawn|GetController))
  (Utilities|Casting|CastToBP_ThirdPersonCharacter Actor)
  (if (.bSuccessfullySensed (Utilities|Struct|BreakAIStimulus Stimulus))
    (bind _asbp_enemy_aicontroller (Utilities|Casting|CastToBP_EnemyAIController _returnvalue))
    (AI|Components|Blackboard|SetValueasObject (Variables|/Script/AIModule.AIController|GetBlackboard _asbp_enemy_aicontroller) (Variables|Default|GetKeyname) Actor)
    (else
      (bind _asbp_enemy_aicontroller_2 (Utilities|Casting|CastToBP_EnemyAIController _returnvalue))
      (AI|Components|Blackboard|ClearValue (Variables|/Script/AIModule.AIController|GetBlackboard _asbp_enemy_aicontroller_2) (Variables|Default|GetKeyname))
      (AI|Components|Blackboard|SetValueasObject (Variables|/Script/AIModule.AIController|GetBlackboard _asbp_enemy_aicontroller_2) (Variables|Default|GetKey%20Name2) (AI|Components|Blackboard|GetValueasObject (Variables|/Script/AIModule.AIController|GetBlackboard _asbp_enemy_aicontroller_2) (Variables|Default|GetKey%20Name2))))))

(event Custom|OnEnemyiDeath
  (Character|LaunchCharacter (* (Transformation|GetActorForwardVector) -5e+02) true true)
  (Utilities|FlowControl|Delay 0.5)
  (Actor|DestroyActor))

(event Custom|OnHitByPlayer
  (params (Hit%20Direction :type Vector))
  (Default|RemoveHealth (Variables|Default|GetHealthComponent) (Variables|Default|GetDamage)))

(event Collision|EventActorBeginOverlap
  (params (OtherActor :type Actor%20Object%20Reference))
  (bind _asbp_third_person_character (Utilities|Casting|CastToBP_ThirdPersonCharacter OtherActor))
  (Game|Damage|ApplyDamage _asbp_third_person_character (Variables|Default|GetDamage) (Pawn|GetController) 0))

(event EventBeginPlay
  (EventDispatchers|BindEventtoOnDeath (Variables|Default|GetHealthComponent) (delegate Custom|OnEnemyiDeath)))

(fn ConstructionScript)