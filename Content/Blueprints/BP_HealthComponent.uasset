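; Health component that gives its owning actor damage, healing and death.
; Current health starts at the maximum on BeginPlay, and TakeDamage and Heal adjust it, clamped between zero and that maximum.
; When damage brings health to zero, TakeDamage calls OnDeath, which destroys the owning actor outright.
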(event EventBeginPlay
  (Variables|Default|SetCurrentHealth (Variables|Default|GetMaxhealth)))

(event EventOnDeath
  (Actor|DestroyActor (Components|GetOwner)))

(fn TakeDamage
  (params (DamageAmount :type Float%20%28double-precision%29))
  (bind _output_get (Variables|Default|SetCurrentHealth (- (Variables|Default|GetCurrentHealth) DamageAmount)))
  (bind _output_get_2 (Variables|Default|SetCurrentHealth (Math|Float|Clamp(Float) _output_get 0.0 (Variables|Default|GetMaxhealth))))
  (if (<= _output_get_2 0.0)
    (CallFunction|OnDeath)))

(fn Heal
  (params (HealAmount :type Float%20%28double-precision%29))
  (bind _output_get (Variables|Default|SetCurrentHealth (+ HealAmount (Variables|Default|GetCurrentHealth))))
  (Variables|Default|SetCurrentHealth (Math|Float|Clamp(Float) _output_get 0.0 (Variables|Default|GetMaxhealth))))