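; Pickable object actor that the third-person character can pick up and drop.
; Box overlap registers it as the character's CurrentInteractable and caches that player, and leaving clears the registration.
; Interact toggles on IsHeld: PickUp disables mesh physics and attaches to the player's HoldPoint.
; Drop re-enables physics but calls DetachFromActor on the cached player rather than on itself.
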(event OnComponentBeginOverlap(Box)
  (params (OverlappedComponent :type Primitive%20Component%20Object%20Reference) (OtherActor :type Actor%20Object%20Reference) (OtherComp :type Primitive%20Component%20Object%20Reference) (OtherBodyIndex :type Integer) (bFromSweep :type Boolean) (SweepResult :type Hit%20Result%20Structure%20%28by%20ref%29))
  (bind _asbp_third_person_character (Utilities|Casting|CastToBP_ThirdPersonCharacter OtherActor))
  (Variables|/Game/ThirdPerson/Blueprints/BP_ThirdPersonCharacter.BP_ThirdPersonCharacter_C|SetCurrentInteractable _asbp_third_person_character self)
  (Variables|Default|SetPlayerRef _asbp_third_person_character))

(event OnComponentEndOverlap(Box)
  (params (OverlappedComponent :type Primitive%20Component%20Object%20Reference) (OtherActor :type Actor%20Object%20Reference) (OtherComp :type Primitive%20Component%20Object%20Reference) (OtherBodyIndex :type Integer))
  (bind _asbp_third_person_character (Utilities|Casting|CastToBP_ThirdPersonCharacter OtherActor))
  (Variables|/Game/ThirdPerson/Blueprints/BP_ThirdPersonCharacter.BP_ThirdPersonCharacter_C|SetCurrentInteractable _asbp_third_person_character 0))

(event EventInteract
  (if (Variables|Default|GetisHeld)
    (CallFunction|Drop)
    (else
      (CallFunction|PickUp))))

(fn ConstructionScript)

(fn Drop
  (Transformation|DetachFromActor (Variables|Default|GetPlayerRef) "KeepRelative" "KeepRelative" "KeepRelative")
  (Physics|SetSimulatePhysics (Variables|Default|GetStaticMesh) true)
  (Variables|Default|SetisHeld false))

(fn PickUp
  (Variables|Default|SetisHeld true)
  (Physics|SetSimulatePhysics (Variables|Default|GetStaticMesh) false)
  (Transformation|AttachComponentToComponent (Variables|/Game/ThirdPerson/Blueprints/BP_ThirdPersonCharacter.BP_ThirdPersonCharacter_C|GetHoldPoint (Variables|Default|GetPlayerRef)) "None" "SnapToTarget" "SnapToTarget" "KeepWorld" true))