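; BP_Crystal is a collectible pickup that counts toward the player's win condition.
; When a BP_ThirdPersonCharacter overlaps its Box, it increments that character's CrystalsCollected, updates the HUD through PlayerHUDref and destroys itself.
; At five or more crystals it also prints a Spanish win message and calls WinGame on the character after a short Delay, both sequenced after its own DestroyActor.
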(event OnComponentBeginOverlap(Box)
  (params (OverlappedComponent :type Primitive%20Component%20Object%20Reference) (OtherActor :type Actor%20Object%20Reference) (OtherComp :type Primitive%20Component%20Object%20Reference) (OtherBodyIndex :type Integer) (bFromSweep :type Boolean) (SweepResult :type Hit%20Result%20Structure%20%28by%20ref%29))
  (bind _asbp_third_person_character (Utilities|Casting|CastToBP_ThirdPersonCharacter OtherActor))
  (bind _output_get (Variables|/Game/ThirdPerson/Blueprints/BP_ThirdPersonCharacter.BP_ThirdPersonCharacter_C|SetCrystalsCollected _asbp_third_person_character (+ (Variables|/Game/ThirdPerson/Blueprints/BP_ThirdPersonCharacter.BP_ThirdPersonCharacter_C|GetCrystalsCollected _asbp_third_person_character) 1)))
  (Default|UpdateCrystals (Variables|/Game/ThirdPerson/Blueprints/BP_ThirdPersonCharacter.BP_ThirdPersonCharacter_C|GetPlayerHUDref _asbp_third_person_character) _output_get)
  (if (>= _output_get 5)
    (Actor|DestroyActor)
    (Development|PrintString "HAS GANADO" true true "(R=0.000000,G=1.000000,B=0.137479,A=1.000000)")
    (Utilities|FlowControl|Delay 2.0)
    (Default|WinGame _asbp_third_person_character)
    (else
      (Actor|DestroyActor))))

(event EventBeginPlay)

(event Collision|EventActorBeginOverlap
  (params (OtherActor :type Actor%20Object%20Reference)))

(event EventTick
  (params (DeltaSeconds :type Float%20%28single-precision%29)))

(fn ConstructionScript)