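; BP_Lever is an interactable lever that toggles a set of receiver objects on and off.
; Its Box overlap sets itself as the third-person character's CurrentInteractable and clears that reference when the overlap ends.
; Interact alternates through a FlipFlop, sending switch-on or switch-off messages to every entry in Receivers and updating IsOn inside each loop.
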(event OnComponentBeginOverlap(Box)
  (params (OverlappedComponent :type Primitive%20Component%20Object%20Reference) (OtherActor :type Actor%20Object%20Reference) (OtherComp :type Primitive%20Component%20Object%20Reference) (OtherBodyIndex :type Integer) (bFromSweep :type Boolean) (SweepResult :type Hit%20Result%20Structure%20%28by%20ref%29))
  (bind _asbp_third_person_character (Utilities|Casting|CastToBP_ThirdPersonCharacter OtherActor))
  (Variables|/Game/ThirdPerson/Blueprints/BP_ThirdPersonCharacter.BP_ThirdPersonCharacter_C|SetCurrentInteractable _asbp_third_person_character self))

(event OnComponentEndOverlap(Box)
  (params (OverlappedComponent :type Primitive%20Component%20Object%20Reference) (OtherActor :type Actor%20Object%20Reference) (OtherComp :type Primitive%20Component%20Object%20Reference) (OtherBodyIndex :type Integer))
  (bind _asbp_third_person_character (Utilities|Casting|CastToBP_ThirdPersonCharacter OtherActor))
  (Variables|/Game/ThirdPerson/Blueprints/BP_ThirdPersonCharacter.BP_ThirdPersonCharacter_C|SetCurrentInteractable _asbp_third_person_character 0))

(event EventInteract
  (Utilities|FlowControl|FlipFlop
    (:A
      (for _array_element (Variables|Default|GetReceivers)
        (Class|ISignalReceiver|Switchon(Message) _array_element)
        (Variables|Default|SetIsOn true)))
    (:B
      (for _array_element_2 (Variables|Default|GetReceivers)
        (Class|ISignalReceiver|SwitchOff(Message) _array_element_2)
        (Variables|Default|SetIsOn false)))))

(fn ConstructionScript)