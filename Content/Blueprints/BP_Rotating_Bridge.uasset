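; BP_Rotating_Bridge is a bridge actor that yaws its root toward 90 degrees past CurrentRotation when switched on.
; A timeline drives the turn by lerping from CurrentRotation to the target rotation.
; Type A bridges play the timeline on switch-on and reverse it on switch-off.
; Other bridges ignore switch-off and play from the start on switch-on, using an IsMoving flag to block retriggering until the timeline finishes.
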(event EventSwitchon
  (Variables|Default|SetTargetRotation (Math|Rotator|MakeRotator 0.0 0.0 (+ (.yaw (Variables|Default|GetCurrentRotation)) 9e+01)))
  (if (Variables|Default|GetIsTypeA)
    (bind _alpha (Timeline|TL_Bridge Play)
      (:Update
        (Transformation|SetRelativeRotation (Variables|Default|GetDefaultSceneRoot) (Math|Rotator|Lerp(Rotator) (Variables|Default|GetCurrentRotation) (Variables|Default|GetTargetRotation) _alpha) false false))
      (:Finished
        (Variables|Default|SetIsMoving false)))
    (elif (not (Variables|Default|GetIsMoving))
      (Variables|Default|SetIsMoving true)
      (Timeline|TL_Bridge PlayFromStart))))

(event EventSwitchOff
  (if (Variables|Default|GetIsTypeA)
    (bind _alpha (Timeline|TL_Bridge Reverse)
      (:Update
        (Transformation|SetRelativeRotation (Variables|Default|GetDefaultSceneRoot) (Math|Rotator|Lerp(Rotator) (Variables|Default|GetCurrentRotation) (Variables|Default|GetTargetRotation) _alpha) false false))
      (:Finished
        (Variables|Default|SetIsMoving false)))))

(fn ConstructionScript)