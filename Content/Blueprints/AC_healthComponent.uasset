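; An actor component that tracks an owner's health and death state.
; RemoveHealth clamps health at zero, broadcasts OnHealthChanged, and on reaching zero sets IsDead and fires OnDeath once, ignoring further damage.
; AddHealth clamps healing to MaxHealth and broadcasts the change, without checking or clearing IsDead.
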(event EventBeginPlay)

(event EventTick
  (params (DeltaSeconds :type Float%20%28single-precision%29)))

(fn RemoveHealth
  (params (Amount :type Float%20%28double-precision%29))
  (if (not (Variables|Default|GetIsDead))
    (bind _output_get (Variables|Default|SetCurrentHealth (Math|Float|Max(Float) (- (Variables|Default|GetCurrentHealth) Amount) 0.0)))
    (Default|CallOnHealthChanged _output_get (Variables|Default|GetMaxHealth))
    (if (<= (Variables|Default|GetCurrentHealth) 0.0)
      (Variables|Default|SetIsDead true)
      (Default|CallOnDeath))))

(fn AddHealth
  (params (Amount :type Float%20%28double-precision%29))
  (bind _output_get (Variables|Default|SetCurrentHealth (Math|Float|Min(Float) (+ (Variables|Default|GetCurrentHealth) Amount) (Variables|Default|GetMaxHealth))))
  (Default|CallOnHealthChanged _output_get (Variables|Default|GetMaxHealth)))